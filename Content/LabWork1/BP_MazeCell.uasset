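; BP_MazeCell is a maze cell that may reveal a random damage-over-time, stake or swinging-axe trap at BeginPlay.
; The construction script sizes the floor and builds optional walls, ceiling and point light from grid settings.
; Trap collisions set damage flags on BP_ThirdPersonGameMode, destroy the floor for stakes or start looping axe Timelines.
; Looping timers poll trap flags and recolor the light from the game mode's TimeUp and Finish states.
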(event `axe1`
  (bind (_direction _newtrack_0) (`Timeline|Timeline` :!label _label)
    (:`Update`
      (`SceneComponent.K2_SetRelativeRotation` (`self.axe01`) (`KismetMathLibrary.RLerp` (struct :`Pitch` 150.0 :`Yaw` 90.0) (struct :`Pitch` 210.0 :`Yaw` 90.0) _newtrack_0) false false))
    (:`Finished`
      (if true
        (goto _label :!via `PlayFromStart`)))))

(event `self.ReceiveBeginPlay`
  (bind _gamemode (`self.gamemode`))
  (bind _asbp_third_person_game_mode (cast `/Game/ThirdPerson/Blueprints/BP_ThirdPersonGameMode` (`GameplayStatics.GetGameMode`)))
  (set `self.gamemode` _asbp_third_person_game_mode)
  (`/Game/ThirdPerson/Blueprints/BP_ThirdPersonGameMode.TimerAndColor` _gamemode 0.0 (struct :`R` 1.0 :`G` 0.007519 :`A` 1.0) (struct :`R` 0.159997 :`G` 1.0 :`A` 1.0))
  (add `/Game/ThirdPerson/Blueprints/BP_ThirdPersonGameMode.TimerAndColor` _gamemode (delegate `TimerAndColor_Event`))
  (`KismetSystemLibrary.K2_SetTimer` null "LightCheck" 0.1 true)
  (`KismetSystemLibrary.K2_SetTimer` null "stakess" 0.5 true)
  (`KismetSystemLibrary.K2_SetTimer` null "axeSwinging" 0.1 true)
  (`KismetSystemLibrary.K2_SetTimer` null "axeCheck" 0.1 true)
  (`self.Trap Type` (`KismetMathLibrary.RandomIntegerInRange` 0 3)))

(event `TimerAndColor_Event`
  (params (Time :type "Float (double-precision)") (Red :type "LinearColor Structure") (GreenColor :type "LinearColor Structure")))

(event `LightCheck`
  (bind _light (`self.light`))
  (if (`/Game/ThirdPerson/Blueprints/BP_ThirdPersonGameMode.timeUp` (`self.gamemode`))
    (`LightComponent.SetLightColor` _light (stale `TimerAndColor_Event` Red) true)
    (elif (`/Game/ThirdPerson/Blueprints/BP_ThirdPersonGameMode.finish` (`self.gamemode`))
      (`LightComponent.SetLightColor` _light (stale `TimerAndColor_Event` GreenColor) true))))

(event `axeCheck`
  (if (`self.SwingTheAxe`)
    (`self.axe1`)
    (`self.axe2`)))

(event `axe2`
  (bind (_direction _newtrack_0) (`Timeline|Timeline_0` :!label _label_2)
    (:`Update`
      (`SceneComponent.K2_SetRelativeRotation` (`self.axe02`) (`KismetMathLibrary.RLerp` (struct :`Pitch` 150.0 :`Yaw` 90.0) (struct :`Pitch` 210.0 :`Yaw` 90.0) _newtrack_0) false false))
    (:`Finished`
      (if true
        (goto _label_2 :!via `PlayFromStart`)))))

(event `stakess`
  (if (`self.Stakes`)
    (`/Engine/EditorBlueprintResources/StandardMacros.DoOnce` false
      (:`Completed`
        (`ActorComponent.K2_DestroyComponent` (`self.Floor`))))))

(event `self.Dot trap.OnComponentBeginOverlap`
  (params (OverlappedComponent :type "PrimitiveComponent Object Reference") (OtherActor :type "Actor Object Reference") (OtherComp :type "PrimitiveComponent Object Reference") (OtherBodyIndex :type Integer) (bFromSweep :type Boolean) (SweepResult :type "HitResult Structure (by ref)"))
  (`KismetSystemLibrary.Delay` 0.5)
  (set `/Game/ThirdPerson/Blueprints/BP_ThirdPersonGameMode.canDamageOT` true (`self.gamemode`)))

(event `self.Dot trap.OnComponentEndOverlap`
  (params (OverlappedComponent :type "PrimitiveComponent Object Reference") (OtherActor :type "Actor Object Reference") (OtherComp :type "PrimitiveComponent Object Reference") (OtherBodyIndex :type Integer))
  (set `/Game/ThirdPerson/Blueprints/BP_ThirdPersonGameMode.canDamageOT` false (`self.gamemode`)))

(event `self.Cube2.OnComponentHit`
  (params (HitComponent :type "PrimitiveComponent Object Reference") (OtherActor :type "Actor Object Reference") (OtherComp :type "PrimitiveComponent Object Reference") (NormalImpulse :type "Vector Structure") (Hit :type "HitResult Structure (by ref)"))
  (set `self.Stakes` true))

(event `self.Cube.OnComponentHit`
  (params (HitComponent :type "PrimitiveComponent Object Reference") (OtherActor :type "Actor Object Reference") (OtherComp :type "PrimitiveComponent Object Reference") (NormalImpulse :type "Vector Structure") (Hit :type "HitResult Structure (by ref)"))
  (set `self.Stakes` true))

(event `self.Cube3.OnComponentHit`
  (params (HitComponent :type "PrimitiveComponent Object Reference") (OtherActor :type "Actor Object Reference") (OtherComp :type "PrimitiveComponent Object Reference") (NormalImpulse :type "Vector Structure") (Hit :type "HitResult Structure (by ref)"))
  (set `self.Stakes` true))

(event `self.Cube1.OnComponentHit`
  (params (HitComponent :type "PrimitiveComponent Object Reference") (OtherActor :type "Actor Object Reference") (OtherComp :type "PrimitiveComponent Object Reference") (NormalImpulse :type "Vector Structure") (Hit :type "HitResult Structure (by ref)"))
  (set `self.Stakes` true))

(event `self.SM_MERGED_BP_MazeCell_C_39.OnComponentHit`
  (params (HitComponent :type "PrimitiveComponent Object Reference") (OtherActor :type "Actor Object Reference") (OtherComp :type "PrimitiveComponent Object Reference") (NormalImpulse :type "Vector Structure") (Hit :type "HitResult Structure (by ref)"))
  (set `/Game/ThirdPerson/Blueprints/BP_ThirdPersonGameMode.canStakeDamage` true (`self.gamemode`))
  (`KismetSystemLibrary.Delay` 0.2)
  (set `/Game/ThirdPerson/Blueprints/BP_ThirdPersonGameMode.canStakeDamage` false (`self.gamemode`)))

(event `self.ip3.OnComponentBeginOverlap`
  (params (OverlappedComponent :type "PrimitiveComponent Object Reference") (OtherActor :type "Actor Object Reference") (OtherComp :type "PrimitiveComponent Object Reference") (OtherBodyIndex :type Integer) (bFromSweep :type Boolean) (SweepResult :type "HitResult Structure (by ref)"))
  (set `self.SwingTheAxe` true))

(event `self.ip2.OnComponentBeginOverlap`
  (params (OverlappedComponent :type "PrimitiveComponent Object Reference") (OtherActor :type "Actor Object Reference") (OtherComp :type "PrimitiveComponent Object Reference") (OtherBodyIndex :type Integer) (bFromSweep :type Boolean) (SweepResult :type "HitResult Structure (by ref)"))
  (set `self.SwingTheAxe` true))

(event `self.ip1.OnComponentBeginOverlap`
  (params (OverlappedComponent :type "PrimitiveComponent Object Reference") (OtherActor :type "Actor Object Reference") (OtherComp :type "PrimitiveComponent Object Reference") (OtherBodyIndex :type Integer) (bFromSweep :type Boolean) (SweepResult :type "HitResult Structure (by ref)"))
  (set `self.SwingTheAxe` true))

(event `self.ip.OnComponentBeginOverlap`
  (params (OverlappedComponent :type "PrimitiveComponent Object Reference") (OtherActor :type "Actor Object Reference") (OtherComp :type "PrimitiveComponent Object Reference") (OtherBodyIndex :type Integer) (bFromSweep :type Boolean) (SweepResult :type "HitResult Structure (by ref)"))
  (set `self.SwingTheAxe` true))

(event `self.axe02.OnComponentHit`
  (params (HitComponent :type "PrimitiveComponent Object Reference") (OtherActor :type "Actor Object Reference") (OtherComp :type "PrimitiveComponent Object Reference") (NormalImpulse :type "Vector Structure") (Hit :type "HitResult Structure (by ref)"))
  (set `/Game/ThirdPerson/Blueprints/BP_ThirdPersonGameMode.canAxeDamage` true (`self.gamemode`))
  (`KismetSystemLibrary.Delay` 0.2)
  (set `/Game/ThirdPerson/Blueprints/BP_ThirdPersonGameMode.canAxeDamage` false (`self.gamemode`)))

(event `self.axe01.OnComponentHit`
  (params (HitComponent :type "PrimitiveComponent Object Reference") (OtherActor :type "Actor Object Reference") (OtherComp :type "PrimitiveComponent Object Reference") (NormalImpulse :type "Vector Structure") (Hit :type "HitResult Structure (by ref)"))
  (set `/Game/ThirdPerson/Blueprints/BP_ThirdPersonGameMode.canAxeDamage` true (`self.gamemode`))
  (`KismetSystemLibrary.Delay` 0.2)
  (set `/Game/ThirdPerson/Blueprints/BP_ThirdPersonGameMode.canAxeDamage` false (`self.gamemode`)))

(fn `Trap Type`
  (params (WhichType :type Integer))
  (bind _ipp (`self.ipp`))
  (bind _stakearray (`self.StakeArray`))
  (`KismetArrayLibrary.Array_Add` _stakearray (`self.Cube3`))
  (`KismetArrayLibrary.Array_Add` _stakearray (`self.Cube1`))
  (`KismetArrayLibrary.Array_Add` _stakearray (`self.Cube2`))
  (`KismetArrayLibrary.Array_Add` _stakearray (`self.Cube`))
  (`KismetArrayLibrary.Array_Add` _stakearray (`self.SM_MERGED_BP_MazeCell_C_39`))
  (switch `int` WhichType
    (:`0`
      (`SceneComponent.SetHiddenInGame` (`self.Dot trap`) false false)
      (`PrimitiveComponent.SetCollisionProfileName` (`self.Dot trap`) "OverlapAllDynamic" true))
    (:`1`
      (for _array_element (`self.StakeArray`)
        (`SceneComponent.SetHiddenInGame` _array_element false false)
        (for _array_element_2 (`self.StakeArray`)
          (`PrimitiveComponent.SetCollisionProfileName` _array_element_2 "BlockAllDynamic" true))))
    (:`2`
      (`KismetArrayLibrary.Array_Add` _ipp (`self.ip`))
      (`KismetArrayLibrary.Array_Add` _ipp (`self.ip1`))
      (`KismetArrayLibrary.Array_Add` _ipp (`self.ip2`))
      (`KismetArrayLibrary.Array_Add` _ipp (`self.ip3`))
      (for _array_element_3 (`self.ipp`)
        (`SceneComponent.SetHiddenInGame` _array_element_3 false false)
        (for _array_element_4 (`self.ipp`)
          (`PrimitiveComponent.SetCollisionProfileName` _array_element_4 "OverlapAllDynamic" true)
          (`SceneComponent.SetHiddenInGame` (`self.axe02`) false false)
          (`SceneComponent.SetHiddenInGame` (`self.axe01`) false false)
          (`PrimitiveComponent.SetCollisionProfileName` (`self.axe01`) "BlockAllDynamic" true)
          (`PrimitiveComponent.SetCollisionProfileName` (`self.axe02`) "BlockAllDynamic" true))))))

(fn `UserConstructionScript`
  (locals (WallThickness :type "Float (double-precision)") (WallLenght :type "Float (double-precision)"))
  (bind _gridsize (`self.GridSize`))
  (bind _walllenght (`local.WallLenght`))
  (bind _walllenght_2 (`local.WallLenght`))
  (bind _returnvalue (* (`local.WallLenght`) 0.5))
  (set `local.WallLenght` _gridsize)
  (set `local.WallThickness` (* _gridsize 0.1))
  (`SceneComponent.SetRelativeScale3D` (`self.Floor`) (`self.SizetoCubeScale` (`KismetMathLibrary.MakeVector` _walllenght _walllenght (`local.WallThickness`))))
  (if (`self.WestWall`)
    (`AddComponent|NODE_AddStaticMeshComponent-0` :`RelativeTransform` (`KismetMathLibrary.MakeTransform` (0.0 0.0 0.0) (struct) (`self.SizetoCubeScale` (`KismetMathLibrary.MakeVector` (`local.WallLenght`) (`local.WallThickness`) (`self.WallHeight`))))))
  (if (`self.EastWall`)
    (`AddComponent|NODE_AddStaticMeshComponent-1` :`RelativeTransform` (`KismetMathLibrary.MakeTransform` (`KismetMathLibrary.MakeVector` 0.0 (- (`local.WallLenght`) (`local.WallThickness`))) (struct) (`self.SizetoCubeScale` (`KismetMathLibrary.MakeVector` (`local.WallLenght`) (`local.WallThickness`) (`self.WallHeight`))))))
  (if (`self.SouthWall`)
    (`AddComponent|NODE_AddStaticMeshComponent-2` :`RelativeTransform` (`KismetMathLibrary.MakeTransform` (0.0 0.0 0.0) (struct) (`self.SizetoCubeScale` (`KismetMathLibrary.MakeVector` (`local.WallThickness`) (`local.WallLenght`) (`self.WallHeight`))))))
  (if (`self.NorthWall`)
    (`AddComponent|NODE_AddStaticMeshComponent-3` :`RelativeTransform` (`KismetMathLibrary.MakeTransform` (`KismetMathLibrary.MakeVector` (- (`local.WallLenght`) (`local.WallThickness`))) (struct) (`self.SizetoCubeScale` (`KismetMathLibrary.MakeVector` (`local.WallThickness`) (`local.WallLenght`) (`self.WallHeight`))))))
  (if (`self.Ceiling`)
    (`AddComponent|NODE_AddStaticMeshComponent-5` :`RelativeTransform` (`KismetMathLibrary.MakeTransform` (`KismetMathLibrary.MakeVector` 0.0 0.0 (- (`local.WallLenght`) (`local.WallThickness`))) (struct) (`self.SizetoCubeScale` (`KismetMathLibrary.MakeVector` _walllenght_2 _walllenght_2 (`local.WallThickness`))))))
  (if (> (`self.LightIntensity`) 0.0)
    (bind _returnvalue_2 (`AddComponent|NODE_AddPointLightComponent-0` :`RelativeTransform` (`KismetMathLibrary.MakeTransform` (`KismetMathLibrary.MakeVector` _returnvalue _returnvalue (* (`self.WallHeight`) 0.75)))))
    (set `self.light` _returnvalue_2)
    (`LightComponent.SetIntensity` _returnvalue_2 (`self.LightIntensity`))
    (`LightComponent.SetLightColor` _returnvalue_2 (`self.LightColor`) true)))